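; BP_Lever is an interactable lever that toggles on Interact_Event and plays a lever sound at its location.
; Tick interpolates the handle's relative rotation between rest and a rolled position based on IsActive.
; Each interaction activates the linked VFX if it is a BP_WaterFountain, then triggers the Affector's BP_WaterCylinder lever event after a three-second delay.
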(event `self.ReceiveTick`
  (params (DeltaSeconds :type "Float (single-precision)"))
  (`SceneComponent.K2_SetRelativeRotation` (`self.Lever_Handle`) (`KismetMathLibrary.RInterpTo` (`SceneComponent.RelativeRotation` (`self.Lever_Handle`)) (select `bool` (`self.isActive`) :`true` (`KismetMathLibrary.MakeRotator` 120.0)) DeltaSeconds (`self.Interp Speed`)) false false))

(event `Interact_Event`
  (set `self.isActive` (not (`self.isActive`)))
  (`GameplayStatics.PlaySoundAtLocation` "/Game/Audio/719586__randomguywhoneverasked__lever.719586__randomguywhoneverasked__lever" (`self.K2_GetActorLocation`) (struct) 1.0 1.0 0.0 null null null null)
  (bind _asbp_water_fountain (cast `/Game/Blueprints/BP_WaterFountain` (`self.VFX`))
    (:`then`
      (`/Game/Blueprints/BP_WaterFountain.Activate_Event` _asbp_water_fountain))
    (:`CastFailed`
      _))
  (bind _asbp_water_cylinder (cast `/Game/Custom/WaterWay/Water/BP_WaterCylinder` (`self.Affector`)))
  (`KismetSystemLibrary.Delay` 3.0)
  (`/Game/Custom/WaterWay/Water/BP_WaterCylinder.Lever_Trigger_Event` _asbp_water_cylinder))

(fn `UserConstructionScript`)