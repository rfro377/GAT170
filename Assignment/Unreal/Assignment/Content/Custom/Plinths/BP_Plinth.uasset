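; Plinth actor that accepts a BP_MagicCube on overlap and triggers an event on its linked EffectTarget.
; On overlap it disables the cube's interaction overlaps, attaches it above the plinth and plays a glow sound at the target's location.
; Tick bobs the cube on a sine wave and spins its box frame per tick, while resetting the inner mesh's world rotation to keep it still.
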(event `self.ReceiveActorBeginOverlap`
  (params (OtherActor :type "Actor Object Reference"))
  (bind _effecttarget (`self.EffectTarget`))
  (bind _asbp_magic_cube (cast `/Game/Custom/MagicCube/BP_MagicCube` OtherActor))
  (bind _output_get (set `self.MagicCubeRef` _asbp_magic_cube))
  (bind _interactioncollider (`/Game/Custom/MagicCube/BP_MagicCube.InteractionCollider` _output_get))
  (set `PrimitiveComponent.bGenerateOverlapEvents` false _interactioncollider)
  (`PrimitiveComponent.SetCollisionObjectType` _interactioncollider "ECC_WorldStatic")
  (`self.K2_AttachToActor` _asbp_magic_cube self "None" "KeepRelative" "KeepRelative" "KeepRelative" true)
  (`GameplayStatics.PlaySoundAtLocation` "/Game/Audio/752274__ienba__magic-glow.752274__ienba__magic-glow" (`self.K2_GetActorLocation` _effecttarget) (struct) 1.0 1.0 0.0 null null null null)
  (`SceneComponent.K2_SetWorldLocation` (`Actor.RootComponent` _output_get) (+ (`SceneComponent.K2_GetComponentLocation` (`self.StaticMesh`)) (0.0 0.0 100.0)) false false)
  (`/Engine/EditorBlueprintResources/StandardMacros.IsValid` _effecttarget
    (:`Is Valid`
      (`/Game/Custom/Plinths/BP_LightEffect.Trigger_Event` _effecttarget))))

(event `self.ReceiveTick`
  (params (DeltaSeconds :type "Float (single-precision)"))
  (bind _magiccuberef (`self.MagicCubeRef`))
  (bind _sm_box (`/Game/Custom/MagicCube/BP_MagicCube.SM_Box` _magiccuberef))
  (bind _sm_box_2 (`/Game/Custom/MagicCube/BP_MagicCube.SM_Box` (`self.MagicCubeRef`)))
  (bind _returnvalue (`SceneComponent.GetRelativeTransform` _sm_box))
  (`/Engine/EditorBlueprintResources/StandardMacros.IsValid` _magiccuberef
    (:`Is Valid`
      ;[1 1 1] Floating and Rotating above PLint
      (`SceneComponent.K2_SetRelativeTransform` _sm_box (`KismetMathLibrary.MakeTransform` (`KismetMathLibrary.MakeVector` (.x (.location _returnvalue)) (.y (.location _returnvalue)) (* (`KismetMathLibrary.Sin` (`KismetSystemLibrary.GetGameTimeInSeconds`)) 8.0)) (`KismetMathLibrary.MakeRotator` (+ (.roll (.rotation _returnvalue)) 1.0) (.pitch (.rotation _returnvalue)) (+ (.yaw (.rotation _returnvalue)) 1.0))) false false)
      ;[1 1 1] Has Magic device float vertically while frame spins
      (`SceneComponent.K2_SetRelativeLocation` _sm_box_2 (+ (`SceneComponent.RelativeLocation` _sm_box_2) (0.0 0.0 100.0)) false false)
      (`SceneComponent.K2_SetWorldRotation` :`self` (`/Game/Custom/MagicCube/BP_MagicCube.SM_MagicCube` (`self.MagicCubeRef`))))))

(fn `UserConstructionScript`)