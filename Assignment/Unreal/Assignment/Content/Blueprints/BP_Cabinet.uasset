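; Interactable cabinet actor with two doors that open and close independently.
; Interact_Event compares the hit component's name to the left and right interact components to choose which door to toggle.
; MoveComponentTo swings that door 90 degrees outward or back to zero, eased over the OverTime duration.
; Door01 sound plays on each toggle, and Door02 follows once a closing move finishes.
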(event `self.ReceiveTick`
  (params (DeltaSeconds :type "Float (single-precision)")))

(event `Interact_Event`
  (params (`Hit Component` :type "PrimitiveComponent Object Reference (by ref)"))
  (bind _returnvalue (`KismetSystemLibrary.GetObjectName` `Hit Component`))
  (bind _over_time (`self.Over Time`))
  (bind _doorl (`self.DoorL`))
  (bind _doorr (`self.DoorR`))
  (if (== _returnvalue "LeftDoorInteract")
    (bind _output_get (set `self.bDoorLOpen` (not (`self.bDoorLOpen`))))
    (if true
      (`GameplayStatics.PlaySound2D` "/Game/Audio/Door/Door-01.Door-01" 1.0 1.0 0.0 null null))
    (`KismetSystemLibrary.MoveComponentTo` _doorl (`SceneComponent.RelativeLocation` _doorl) (select `bool` _output_get :`true` (`KismetMathLibrary.MakeRotator` 0.0 0.0 -90.0)) true true _over_time)
    (if (not (`self.bDoorLOpen`))
      (`GameplayStatics.PlaySound2D` "/Game/Audio/Door/Door-02.Door-02" 1.0 1.0 0.0 null null))
    (elif (== _returnvalue "RightDoorInteract")
      (bind _output_get_2 (set `self.bDoorROpen` (not (`self.bDoorROpen`))))
      (if true
        (`GameplayStatics.PlaySound2D` "/Game/Audio/Door/Door-01.Door-01" 1.0 1.0 0.0 null null))
      (`KismetSystemLibrary.MoveComponentTo` _doorr (`SceneComponent.RelativeLocation` _doorr) (select `bool` _output_get_2 :`true` (`KismetMathLibrary.MakeRotator` 0.0 0.0 90.0)) true true _over_time)
      (if (not (`self.bDoorROpen`))
        (`GameplayStatics.PlaySound2D` "/Game/Audio/Door/Door-02.Door-02" 1.0 1.0 0.0 null null)))))

(fn `UserConstructionScript`)