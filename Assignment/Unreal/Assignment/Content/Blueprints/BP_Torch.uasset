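; BP_Torch is an interactable torch actor that toggles on and off, starting unlit.
; Interact_Event flips IsOn, plays a fire burst sound at the torch and starts or stops the looping-style crackle audio.
; Tick flickers the point light intensity with a sine of game time and syncs light and flame effect visibility to IsOn.
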(event `self.ReceiveBeginPlay`
  (set `self.isOn` false))

(event `self.ReceiveTick`
  (params (DeltaSeconds :type "Float (single-precision)"))
  (bind _ison (`self.isOn`))
  (`LightComponent.SetIntensity` (`self.PointLight`) (+ (* (`KismetMathLibrary.DegSin` (* (`KismetSystemLibrary.GetGameTimeInSeconds`) (`self.TimeMultiplier`))) (`self.LightIntensity Multiplier`)) (`self.Base Intensity`)))
  (`SceneComponent.SetVisibility` (`self.PointLight`) _ison false)
  (`SceneComponent.SetVisibility` (`self.NS_TorchFlame`) _ison false))

(event `Interact_Event`
  (bind _output_get (set `self.isOn` (not (`self.isOn`))))
  (`GameplayStatics.PlaySoundAtLocation` "/Game/Audio/Torch/435845__fireburst.435845__fireburst" (`self.K2_GetActorLocation`) (struct) 1.0 1.0 0.0 null null null null)
  (if _output_get
    (`AudioComponent.Play` (`self.Firecrackle`) 0.0)
    (else
      (`AudioComponent.Stop` (`self.Firecrackle`)))))

(fn `UserConstructionScript`)