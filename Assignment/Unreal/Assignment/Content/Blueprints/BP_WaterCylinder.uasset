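; BP_WaterCylinder is a water cylinder that alternates between filling and draining each time its lever trigger event fires.
; The event flips IsFilling, starting the water sound when filling and stopping it when draining.
; MoveComponentTo eases the Water component over a fixed duration to the target relative location for filling, or to that location negated for draining.
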(event `self.ReceiveTick`
  (params (DeltaSeconds :type "Float (single-precision)")))

(event `Lever_Trigger_Event`
  (bind _water (`self.Water`))
  (bind _target_relative_location (`self.Target Relative Location`))
  (bind _output_get (set `self.isFilling` (not (`self.isFilling`))))
  (if _output_get
    (`AudioComponent.Play` (`self.WaterSound`) 0.0)
    (`KismetSystemLibrary.MoveComponentTo` _water _target_relative_location (struct) true true 10.0)
    (else
      (`AudioComponent.Stop` (`self.WaterSound`))
      (`KismetSystemLibrary.MoveComponentTo` _water (* _target_relative_location -1.0) (struct) true true 10.0))))

(fn `UserConstructionScript`)