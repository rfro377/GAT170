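; BP_LightEffect is an actor that pairs a Glow light with a Niagara effect that can be switched on by an event.
; Trigger_Event shows the light, activates the particle system and sets a high target intensity and interpolation speed.
; Tick eases the light's intensity toward that target every frame with FInterpTo.
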(event `self.ReceiveTick`
  (params (DeltaSeconds :type "Float (single-precision)"))
  (bind _glow (`self.Glow`))
  (`LightComponent.SetIntensity` _glow (`KismetMathLibrary.FInterpTo` (`LightComponentBase.Intensity` _glow) (`self.TargetIntensity`) DeltaSeconds (`self.Interp Speed`))))

(event `Trigger_Event`
  (`SceneComponent.SetVisibility` (`self.Glow`) true false)
  (`ActorComponent.SetActive` (`self.Niagara`) true false)
  (set `self.TargetIntensity` 40000.0)
  (set `self.Interp Speed` 5.0))

(fn `UserConstructionScript`)